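; Tile actor for infinite terrain, with a barrier that locks and unlocks as the player passes through.
; The barrier starts red and solid, turning green and non-colliding while the player overlaps TriggerToLock.
; Leaving that trigger relocks it and asks BP_InfiniteTerrainGameMode to spawn a tile, while entering TriggerToDestroy destroys this one.
; GetAttachLocation exposes the Arrow's world transform as an attach point.
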(event `self.ReceiveBeginPlay`
  (`self.Lock`))

(event `self.TriggerToLock.OnComponentBeginOverlap`
  (params (OverlappedComponent :type "PrimitiveComponent Object Reference") (OtherActor :type "Actor Object Reference") (OtherComp :type "PrimitiveComponent Object Reference") (OtherBodyIndex :type Integer) (bFromSweep :type Boolean) (SweepResult :type "HitResult Structure (by ref)"))
  (`self.IsPlayer` OtherActor
    (:`true`
      (`self.Unlock`))))

(event `self.TriggerToLock.OnComponentEndOverlap`
  (params (OverlappedComponent :type "PrimitiveComponent Object Reference") (OtherActor :type "Actor Object Reference") (OtherComp :type "PrimitiveComponent Object Reference") (OtherBodyIndex :type Integer))
  (`self.IsPlayer` OtherActor
    (:`true`
      (`self.Lock`)
      (bind _asbp_infinite_terrain_game_mode (cast `/Game/Blueprints/GameMode/BP_InfiniteTerrainGameMode` (`GameplayStatics.GetGameMode`)))
      (`/Game/Blueprints/GameMode/BP_InfiniteTerrainGameMode.SpawnTile` _asbp_infinite_terrain_game_mode))))

(event `self.TriggerToDestroy.OnComponentBeginOverlap`
  (params (OverlappedComponent :type "PrimitiveComponent Object Reference") (OtherActor :type "Actor Object Reference") (OtherComp :type "PrimitiveComponent Object Reference") (OtherBodyIndex :type Integer) (bFromSweep :type Boolean) (SweepResult :type "HitResult Structure (by ref)"))
  (`self.IsPlayer` OtherActor
    (:`true`
      (`self.K2_DestroyActor`))))

(fn `GetAttachLocation`
  (returns (`Attach Transform` :type "Transform Structure"))
  (return (`SceneComponent.K2_GetComponentToWorld` (`self.Arrow`))))

(fn `Lock`
  (bind _barrier (`self.Barrier`))
  (`PrimitiveComponent.SetMaterial` _barrier 0 "/Game/Geometry/Materials/TransRed_Inst.TransRed_Inst")
  (`PrimitiveComponent.SetCollisionEnabled` _barrier "QueryAndPhysics"))

(fn `Unlock`
  (bind _barrier (`self.Barrier`))
  (`PrimitiveComponent.SetMaterial` _barrier 0 "/Game/Geometry/Materials/TransGreen_Inst.TransGreen_Inst")
  (`PrimitiveComponent.SetCollisionEnabled` _barrier "NoCollision"))

(fn `UserConstructionScript`)