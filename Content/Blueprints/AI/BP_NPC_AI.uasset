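; BP_NPC_AI is an AI controller that drives a guard NPC and detects the player.
; On BeginPlay it loads the PatrolData blackboard, runs the BT_GuardBehaviour tree and caches the controlled BP_Character.
; AI perception updates set EnemyKey to the player pawn when sensed and clear it when sight or other stimulus is lost, feeding the behavior tree.
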(event `self.ReceiveBeginPlay`
  (bind _blackboardcomponent (`self.UseBlackboard` "/Game/Blueprints/AI/PatrolData.PatrolData"))
  (set `self.BlackboardComp` _blackboardcomponent)
  (`self.RunBehaviorTree` "/Game/Blueprints/AI/BehaviourTree/BT_GuardBehaviour.BT_GuardBehaviour")
  (bind _asbp_character (cast `/Game/Blueprints/Character/BP_Character` (`self.K2_GetPawn`)))
  (set `self.TPCharacter` _asbp_character))

(event `self.AIPerception.OnTargetPerceptionUpdated`
  (params (Actor :type "Actor Object Reference") (Stimulus :type "AIStimulus Structure"))
  (bind _blackboardcomp (`self.BlackboardComp`))
  (bind _enemykey (`self.EnemyKey`))
  (if (== (`GameplayStatics.GetPlayerPawn` 0) Actor)
    (if (`.bSuccessfullySensed` (break `AIStimulus` Stimulus))
      (`BlackboardComponent.SetValueAsObject` _blackboardcomp _enemykey Actor)
      (else
        (`BlackboardComponent.ClearValue` _blackboardcomp _enemykey)))))

(fn `UserConstructionScript`)